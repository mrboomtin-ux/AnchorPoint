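; Blueprint function library for the character's grapple: it attaches the cable to the nearest anchor and drives swing movement.
; SwingMovement adds force toward the anchor, using centripetal force (mass × velocity² / distance) scaled by how much velocity points away from it.
; A tension curve over normalized distance filters that force, with slight damping compensation.
; The constant pull term is currently multiplied by zero.
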(fn ConnectCable&Anchor
  (params (Actor :type %20Object%20Reference) (__WorldContext :type Object%20Object%20Reference))
  (Variables|/Script/CableComponent.CableComponent|SetEndLocation (Variables|Default|GetCable Actor) (Math|Transform|InverseTransformLocation (Transformation|GetActorTransform Actor) (Transformation|GetActorLocation (Variables|Default|GetNearest%20Anchor Actor))))
  (return))

(fn CalculateCentripetalForce
  (params (Distance%20from%20Center :type Float%20%28double-precision%29) (Actor :type %20Object%20Reference) (__WorldContext :type Object%20Object%20Reference))
  (return (* (/ (Math|Vector|VectorLengthSquared (Transformation|GetVelocity Actor)) Distance%20from%20Center) (Variables|Default|GetMass Actor))))

(fn SwingMovement
  (params (Actor :type %20Object%20Reference) (__WorldContext :type Object%20Object%20Reference))
  (bind _returnvalue (Transformation|GetActorLocation Actor))
  (bind _grappletensioncurve (Variables|Default|GetGrappleTensionCurve Actor))
  (bind _nearest_anchor (Variables|Default|GetNearest%20Anchor Actor))
  (bind _returnvalue_2 (Transformation|GetActorLocation _nearest_anchor))
  (bind _returnvalue_3 (Math|Vector|GetUnitDirection(Vector) _returnvalue _returnvalue_2))
  (bind _returnvalue_4 (Math|Vector|Distance(Vector) _returnvalue _returnvalue_2))
  (bind _returnvalue_5 (Math|Float|NormalizetoRange _returnvalue_4 0.0 4e+02))
  (bind _returnvalue_6 (Class|KismetMathLibrary|GetRuntimeFloatCurveValue _grappletensioncurve _returnvalue_5 0.0))
  ;[0.15 0.15 0.15 0.5] Swinging Mechanic
  (Physics|AddForce (Variables|/Script/Engine.Character|GetCharacterMovement Actor) (* _returnvalue_3 (* (+ (* _returnvalue_6 0.0) (* _returnvalue_6 (* (CallFunction|CalculateCentripetalForce _returnvalue_4 Actor) (Math|Float|Clamp(Float) (Math|Vector|DotProduct _returnvalue_3 (Math|Vector|NegateVector (Math|Vector|Normalize (Transformation|GetVelocity Actor)))) 0.01)))) 1.02))))