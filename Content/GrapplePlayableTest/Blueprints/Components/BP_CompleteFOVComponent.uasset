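; An actor component that widens or narrows its owner's camera field of view with movement speed.
; On BeginPlay it caches the first actor of the owner's class, found via GetActorOfClass rather than using the owner directly, and that actor's CameraComponent.
; Each Tick maps velocity magnitude between editable speed limits onto an FOV range, then eases the camera toward it with FInterpTo at a fixed rate.
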(event EventBeginPlay
  ;[0.15 0.15 0.15 0.5] Get a reference to the character this component is attached to.
  (bind _returnvalue (Actor|GetActorOfClass (Utilities|GetClass (Components|GetOwner))))
  (Utilities|IsValid _returnvalue
    (:Is%20Valid
      (bind _output_get (Variables|Default|SetPlayerPawn _returnvalue))
      ;[0.15 0.15 0.15 0.5] Get the camera component attached to the owning actor.
      (Utilities|IsValid (Actor|GetComponentbyClass _output_get "/Script/Engine.CameraComponent")
        (:Is%20Valid
          (Variables|Default|SetCamera%20Component (Actor|GetComponentbyClass _output_get "/Script/Engine.CameraComponent")))))))

(event EventTick
  (params (DeltaSeconds :type Float%20%28single-precision%29))
  (bind _camera_component (Variables|Default|GetCamera%20Component))
  ;[0.15 0.15 0.15 0.5] Modify FOV of the camera based on velocity of owner
  (Camera|SetFieldOfView _camera_component (Math|Interpolation|FInterpTo (Variables|/Script/Engine.CameraComponent|GetFieldOfView _camera_component) (Math|Float|MapRangeClamped (Math|Vector|VectorLength (Transformation|GetVelocity (Variables|Default|GetPlayerPawn))) (Variables|Default|GetMin%20Velocity) (Variables|Default|GetMax%20Velocity) (Variables|Default|GetMin%20FOV) (Variables|Default|GetMax%20FOV)) DeltaSeconds 0.8)))