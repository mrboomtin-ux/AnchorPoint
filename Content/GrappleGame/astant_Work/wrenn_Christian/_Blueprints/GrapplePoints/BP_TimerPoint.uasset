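; BP_TimerPoint is a grapple point that only holds the player for a limited time.
; OnGrapple starts the TimitLimit event, which waits half of TimeLimit and then has the grapple character's UI manager show break text.
; After the second half elapses, it fully resets the character's grapple.
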(event Custom|TimitLimit
  (bind _as_bp_grapplechar_ace (Variables|Default|GetAs%20BP%20Grapplechar%20Ace))
  (bind _timelimit (Variables|Default|GetTimeLimit))
  (bind _returnvalue (/ _timelimit 2.0))
  (Utilities|FlowControl|Delay _returnvalue)
  (Default|ActivateBreakText (Variables|/Game/GrappleGame/astant_Work/wrenn_Christian/_Blueprints/BP_GrapplecharAce.BP_GrapplecharAce_C|GetAs%20BP%20UI%20Manager _as_bp_grapplechar_ace))
  (Utilities|FlowControl|Delay _returnvalue)
  (Default|ResetGrappleFully _as_bp_grapplechar_ace))

(fn ConstructionScript
  (|CallParentFunction))

(fn OnGrapple
  (params (InteractingPlayer :type Character%20Object%20Reference))
  (CallFunction|TimitLimit)
  (return "NewEnumerator0"))