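; BP_Checkpoint is a one-shot trigger that updates the player's respawn point in the grapple game.
; When the player's capsule overlaps its box, it passes the RespawnPoint location and the arrow's forward-vector X/Y to BP_LevelManager.
; It then hides itself, shows WBP_Checkpoint for a short delay, and destroys itself.
; The construction script sets the box's size, offset and rotation, plus the arrow's facing, from variables.
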(event OnComponentBeginOverlap(Box)
  (params (OverlappedComponent :type Primitive%20Component%20Object%20Reference) (OtherActor :type Actor%20Object%20Reference) (OtherComp :type Primitive%20Component%20Object%20Reference) (OtherBodyIndex :type Integer) (bFromSweep :type Boolean) (SweepResult :type Hit%20Result%20Structure%20%28by%20ref%29))
  (bind _arrow (Variables|Default|GetArrow))
  (bind _returnvalue (Math|Vector|GetForwardVector _arrow))
  ;[0.15 0.15 0.15 0.5] When the player overlaps the box, set the current respawn point to the Respawn Components location.
  (if (== OtherComp (Variables|/Script/Engine.Character|GetCapsuleComponent (Variables|Default|GetAs%20BP%20Grapple%20Character)))
    (bind _output_get (Variables|Default|SetCurrent%20Respawn%20Position%20Location (Transformation|GetWorldLocation (Variables|Default|GetRespawnPoint))))
    (Default|UpdateRespawnPoint (Variables|Default|GetLevelManagerRef) (Math|Transform|MakeTransform _output_get (Math|Rotator|MakeRotator (.x _returnvalue) (.y _returnvalue) 0.0) "1.000000,1.000000,1.000000"))
    (bind _returnvalue_2 (UserInterface|CreateWidget "/Game/GrappleGame/Progamers/_Blueprints/UI/WBP_Checkpoint.WBP_Checkpoint_C"))
    ;[0.15 0.15 0.15 0.5] hides actor then destroys after setting ui text up
    (Rendering|SetActorHiddenInGame true)
    (UserInterface|Viewport|AddtoViewport _returnvalue_2 0)
    (Utilities|FlowControl|Delay 0.8)
    (Widget|RemovefromParent _returnvalue_2)
    (Actor|DestroyActor)))

(event EventBeginPlay
  ;[0.15 0.15 0.15 0.5] Get reference to the Level Manager
  (bind _returnvalue (Actor|GetActorOfClass "/Game/GrappleGame/Progamers/_Blueprints/PuzzleMechanics/BP_LevelManager.BP_LevelManager_C"))
  (Variables|Default|SetLevelManagerRef _returnvalue)
  ;[0.15 0.15 0.15 0.5] player ref
  (bind _asbp_grapple_character (Utilities|Casting|CastToBP_GrappleCharacter (Game|GetPlayerCharacter 0)))
  (Variables|Default|SetAs%20BP%20Grapple%20Character _asbp_grapple_character))

(fn ConstructionScript
  (Utilities|FlowControl|Sequence
    (:then_0
      (Transformation|AddLocalOffset (Variables|Default|GetBox) (Math|Vector|MakeVector 0.0 0.0 (.z (Variables|Default|GetBox%20Shape))) false false)
      (Components|Box|SetBoxExtent (Variables|Default|GetBox) (Variables|Default|GetBox%20Shape) true)
      (Transformation|SetRelativeRotation (Variables|Default|GetBox) (Variables|Default|GetBoxRotation) false false))
    (:then_1
      (Transformation|SetRelativeRotation (Variables|Default|GetArrow) (Variables|Default|GetRespawnFaceDirection) false false))))