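; Level manager that tracks puzzle gates and the player's respawn point.
; On BeginPlay it maps every BP_Gate to false and stores the BP_GrappleCharacter's location as the initial respawn transform.
; UpdateOpengates scans that map, breaking at the first false value, with the loop's Completed output calling LevelClear, an empty event here.
; UpdateRespawnPoint overwrites the stored respawn transform.
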(event Custom|UpdateRespawnPoint
  (params (CurrentRespawnPosition :type Transform))
  ;[0.04167 0.07554 0.1698 0.5] Store new respawn location
  (Variables|Default|SetCurrentRespawnPosition CurrentRespawnPosition))

(event Custom|UpdateOpengates
  ;[0.04167 0.07554 0.1698 0.5] Check if all gate are open.
  (bind _valuepin (Utilities|Map|ForEachLoop(Map) (Variables|Default|GetLevelGates) :!label _label)
    (:then
      (if (not _valuepin)
        (goto _label BreakPin)))
    (:CompletedPin
      (CallFunction|LevelClear))))

(event Custom|LevelClear)

(event EventBeginPlay
  ;[0.04167 0.07554 0.1698 0.5] Get references to all gates in the level.
  (Utilities|FlowControl|Sequence
    (:then_0
      (bind _outactors (Actor|GetAllActorsOfClass "/Game/GrappleGame/Progamers/_Blueprints/PuzzleMechanics/BP_Gate.BP_Gate_C"))
      (for _array_element _outactors
        (Utilities|IsValid _array_element
          (:Is%20Valid
            (Utilities|Map|Add (Variables|Default|GetLevelGates) _array_element false)))))
    (:then_1
      (bind _asbp_grapple_character (Utilities|Casting|CastToBP_GrappleCharacter (Game|GetPlayerCharacter 0)))
      (Variables|Default|SetCurrentRespawnPosition (Math|Transform|MakeTransform (Transformation|GetActorLocation _asbp_grapple_character) "0, 0, 0" "1.000000,1.000000,1.000000")))))

(fn ConstructionScript)