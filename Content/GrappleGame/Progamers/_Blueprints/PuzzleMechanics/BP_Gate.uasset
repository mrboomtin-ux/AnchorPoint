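; BP_Gate is a puzzle gate that removes itself from the level once enough of its locks are activated.
; The construction script applies the chosen mesh and sizes the Locks array to AmountOfLocks.
; UpdateLocksOpened recounts activated locks and calls OpenGate, which destroys the actor, when the count reaches that amount.
; Nothing here triggers the recount, as the Timeline that would poll it is never run.
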(event Custom|UpdateLocksOpened
  (Variables|Default|SetLocksOpened 0)
  (for _array_element (Variables|Default|GetLocks)
    (if (Variables|/Game/GrappleGame/jahawkins_Work/_BluePrints/InteractableObjects/BP_InteractableObject.BP_InteractableObject_C|GetObjectActivated _array_element)
      (Math|Integer|IncrementInt (Variables|Default|GetLocksOpened))))
  (if (>= (Variables|Default|GetLocksOpened) (Variables|Default|GetAmountOfLocks))
    (CallFunction|OpenGate)))

(event Custom|OpenGate
  (Actor|DestroyActor))

(fn ConstructionScript
  (Components|StaticMesh|SetStaticMesh (Variables|Default|GetStaticMesh) (Variables|Default|GetMesh))
  (Utilities|Array|Resize (Variables|Default|GetLocks) (Variables|Default|GetAmountOfLocks)))