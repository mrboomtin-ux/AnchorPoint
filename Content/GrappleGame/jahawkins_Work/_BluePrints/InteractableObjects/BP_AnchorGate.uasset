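; BP_AnchorGate is a two-door sliding gate that hooks into a linked interactable object or pressure plate.
; BeginPlay saves the doors' placed transforms as open poses and derives closed poses from them with opposite X offsets.
; It casts the linked object to either supported type and binds to its Activate and Deactivate events, printing debug strings.
; OpenGate and CloseGate each play a timeline that lerps both doors between those poses.
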(event Custom|CloseGate
  (bind _alpha (Timeline|T_Close PlayFromStart)
    (:Update
      (Transformation|SetRelativeTransform (Variables|Default|GetDoor_L) (Math|Transform|Lerp(Transform) (Variables|Default|GetL_OpenPos) (Variables|Default|GetL_ClosePos) _alpha) false false)
      (Transformation|SetRelativeTransform (Variables|Default|GetDoor_R) (Math|Transform|Lerp(Transform) (Variables|Default|GetR_OpenPos) (Variables|Default|GetR_ClosePos) _alpha) false false))))

(event Custom|OpenGate
  (bind _alpha (Timeline|T_Open PlayFromStart)
    (:Update
      (Transformation|SetRelativeTransform (Variables|Default|GetDoor_L) (Math|Transform|Lerp(Transform) (Variables|Default|GetL_ClosePos) (Variables|Default|GetL_OpenPos) _alpha) false false)
      (Transformation|SetRelativeTransform (Variables|Default|GetDoor_R) (Math|Transform|Lerp(Transform) (Variables|Default|GetR_ClosePos) (Variables|Default|GetR_OpenPos) _alpha) false false))))

(event EventBeginPlay
  (bind _door_r (Variables|Default|GetDoor_R))
  (bind _door_l (Variables|Default|GetDoor_L))
  (bind _interactableobject (Variables|Components|GetInteractableObject))
  (bind _returnvalue (Transformation|GetRelativeTransform _door_l))
  (bind _returnvalue_2 (Transformation|GetRelativeTransform _door_r))
  (bind (_location _rotation _scale) (Math|Transform|BreakTransform _returnvalue))
  (bind (_location_2 _rotation_2 _scale_2) (Math|Transform|BreakTransform _returnvalue_2))
  (bind (_x _y _z) (Math|Vector|BreakVector _location))
  (bind (_x_2 _y_2 _z_2) (Math|Vector|BreakVector _location_2))
  (Utilities|FlowControl|Sequence
    (:then_0
      (Variables|Default|SetL_OpenPos _returnvalue)
      (Variables|Default|SetL_ClosePos (Math|Transform|MakeTransform (+ _location (Math|Vector|MakeVector (+ _x -2e+02) _y _z)) _rotation _scale)))
    (:then_1
      (Variables|Default|SetR_OpenPos _returnvalue_2)
      (Variables|Default|SetR_ClosePos (Math|Transform|MakeTransform (+ _location_2 (Math|Vector|MakeVector (+ _x_2 2e+02) _y_2 _z_2)) _rotation_2 _scale_2)))
    (:then_2
      (bind _asbp_interactable_object (Utilities|Casting|CastToBP_InteractableObject _interactableobject)
        (:then
          (Development|PrintString "Hello" true true "(R=0.000000,G=1.000000,B=1.000000,A=1.000000)")
          (EventDispatchers|BindEventtoActivate _asbp_interactable_object (EventDispatchers|CreateEvent :!event Custom|CloseGate))
          (EventDispatchers|BindEventtoDeactivate _asbp_interactable_object (EventDispatchers|CreateEvent :!event Custom|OpenGate)))
        (:CastFailed
          (bind _asbp_pressure_plate_v2 (Utilities|Casting|CastToBP_PressurePlateV2 _interactableobject)
            (:then
              (Development|PrintString "Hello" true true "(R=1.000000,G=1.000000,B=0.000000,A=1.000000)")
              (EventDispatchers|BindEventtoActivate _asbp_pressure_plate_v2 (EventDispatchers|CreateEvent :!event Custom|CloseGate))
              (EventDispatchers|BindEventtoDeactivate _asbp_pressure_plate_v2 (EventDispatchers|CreateEvent :!event Custom|OpenGate)))
            (:CastFailed
              (Development|PrintString "Goodbye" true true "(R=1.000000,G=0.000000,B=1.000000,A=1.000000)"))))))))

(fn ConstructionScript)