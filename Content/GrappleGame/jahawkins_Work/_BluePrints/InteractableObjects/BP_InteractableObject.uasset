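; BP_InteractableObject is an interactable object that the player switches on, reporting as interactable and returning its GrappleType when grappled.
; OnInteract triggers Interact, which after a one-tick delay activates an inactive object, changes its color and calls the Activate dispatcher.
; BeginPlay creates a dynamic material for that color feedback and starts the object inactive.
; Deactivation logic, gated by CanDeactivate, exists but is unconnected and never runs.
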(event Custom|Interact
  ;[1 0.15 0 0.5] Player interacts with object (Programmers replace this with the action used.
  (Utilities|FlowControl|DelayUntilNextTick)
  ;[1 0.15 0 0.5] Check if object is activated
  (if (not (Variables|Default|GetObjectActivated))
    ;[1 0.15 0 0.5] Activate object
    (if (Variables|Default|GetObjectActivated)
      (Development|PrintString "ERROR! This object is already activated!" true true "(R=1.000000,G=0.000000,B=0.000000,A=1.000000)" 5.0)
      (else
        (Variables|Default|SetObjectActivated true)
        (Rendering|Material|SetVectorParameterValue (Variables|Default|GetDMI) "color" (Variables|Default|GetActiveColor) :!class /Script/Engine.MaterialInstanceDynamic)
        (Default|CallActivate)))))

(event EventBeginPlay
  (bind _interactable (Variables|Default|GetInteractable))
  ;[1 0.15 0 0.5] Object setup when game starts
  (Utilities|FlowControl|Sequence
    (:then_0
      ;;[1 0.15 0 0.5] Creates a material instance to change the color of the object
      (bind _returnvalue (Rendering|Material|CreateDynamicMaterialInstance _interactable 0 0 "DMI_Cube" :!class /Script/Engine.PrimitiveComponent))
      (bind _output_get (Variables|Default|SetDMI _returnvalue))
      (Rendering|Material|SetMaterial _interactable 0 _output_get))
    (:then_1
      ;;[1 0.15 0 0.5] Set state of object at start
      (Variables|Default|SetObjectActivated false)
      (Rendering|Material|SetVectorParameterValue (Variables|Default|GetDMI) "color" (Variables|Default|GetInctiveColor) :!class /Script/Engine.MaterialInstanceDynamic))))

(fn ConstructionScript)

(fn OnGrapple
  (params (InteractingPlayer :type Character%20Object%20Reference))
  (return (Variables|Default|GetGrappleType)))

(fn OnInteract
  (params (InteractingPlayer :type Character%20Object%20Reference) (Location :type Vector :default "0, 0, 0"))
  (CallFunction|Interact)
  (return "0, 0, 0"))

(fn IsInteractable
  (return true))