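; BP_Gate is a gate that rises 400 units to open and lowers back to its starting position to close.
; On BeginPlay it stores both transforms and binds to the activate and deactivate events of its linked BP_InteractableObject or BP_PressurePlateV2, printing debug strings.
; OpenDoor and CloseDoor use separate timelines to lerp between the transforms, always playing from the start, so an interrupted move jumps to an endpoint.
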(event Custom|CloseDoor
  (bind _alpha (Timeline|T_Close PlayFromStart)
    (:Update
      (Transformation|SetActorTransform (Math|Transform|Lerp(Transform) (Variables|Default|GetOpenPos) (Variables|Default|GetClosedPos) _alpha)))))

(event Custom|OpenDoor
  (bind _alpha (Timeline|T_Open PlayFromStart)
    (:Update
      (Transformation|SetActorTransform (Math|Transform|Lerp(Transform) (Variables|Default|GetClosedPos) (Variables|Default|GetOpenPos) _alpha)))))

(event Collision|EventActorBeginOverlap
  (params (OtherActor :type Actor%20Object%20Reference)))

(event EventTick
  (params (DeltaSeconds :type Float%20%28single-precision%29)))

(event EventBeginPlay
  (bind _returnvalue (Transformation|GetActorTransform))
  (bind _interactableobject (Variables|Components|GetInteractableObject))
  (bind (_location _rotation _scale) (Math|Transform|BreakTransform _returnvalue))
  (bind (_x _y _z) (Math|Vector|BreakVector _location))
  (Variables|Default|SetClosedPos _returnvalue)
  (Variables|Default|SetOpenPos (Math|Transform|MakeTransform (Math|Vector|MakeVector _x _y (+ _z 4e+02)) _rotation _scale))
  (bind _asbp_interactable_object (Utilities|Casting|CastToBP_InteractableObject _interactableobject)
    (:then
      (Development|PrintString "Hello" true true "(R=0.000000,G=1.000000,B=1.000000,A=1.000000)")
      (EventDispatchers|BindEventtoActivate _asbp_interactable_object (EventDispatchers|CreateEvent :!event Custom|OpenDoor))
      (EventDispatchers|BindEventtoDeactivate _asbp_interactable_object (EventDispatchers|CreateEvent :!event Custom|CloseDoor)))
    (:CastFailed
      (bind _asbp_pressure_plate_v2 (Utilities|Casting|CastToBP_PressurePlateV2 _interactableobject)
        (:then
          (Development|PrintString "Hello" true true "(R=1.000000,G=1.000000,B=0.000000,A=1.000000)")
          (EventDispatchers|BindEventtoActivate _asbp_pressure_plate_v2 (EventDispatchers|CreateEvent :!event Custom|OpenDoor))
          (EventDispatchers|BindEventtoDeactivate _asbp_pressure_plate_v2 (EventDispatchers|CreateEvent :!event Custom|CloseDoor)))
        (:CastFailed
          (Development|PrintString "Goodbye" true true "(R=1.000000,G=0.000000,B=1.000000,A=1.000000)"))))))

(fn ConstructionScript)