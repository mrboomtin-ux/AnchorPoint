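; BP_ProxLever is a proximity lever that activates when the grapple character's capsule overlaps its Interactable component.
; Activation latches ObjectActivated, tints a dynamic material instance created at BeginPlay to the active color, and calls Activate; repeat attempts print an error.
; Nothing resets it during play: IO_Deactivate is empty, IsInteractable returns false, and OnGrapple returns a fixed enum value.
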(event OnComponentBeginOverlap(Interactable)
  (params (OverlappedComponent :type Primitive%20Component%20Object%20Reference) (OtherActor :type Actor%20Object%20Reference) (OtherComp :type Primitive%20Component%20Object%20Reference) (OtherBodyIndex :type Integer) (bFromSweep :type Boolean) (SweepResult :type Hit%20Result%20Structure%20%28by%20ref%29))
  ;[1 0.15 0 0.5] Player interacts with object
  (bind _returnvalue (Actor|GetActorOfClass "/Game/GrappleGame/Progamers/_Blueprints/BP_GrappleCharacter.BP_GrappleCharacter_C"))
  (if (Class|PrimitiveComponent|IsOverlappingComponent (Variables|/Script/Engine.Character|GetCapsuleComponent _returnvalue) (Variables|Default|GetInteractable))
    (CallFunction|PPActivate)))

(event Custom|PP_Activate
  ;[1 0.15 0 0.5] Activate object
  (if (Variables|Default|GetObjectActivated)
    (Development|PrintString "ERROR! This object is already activated!" true true "(R=1.000000,G=0.000000,B=0.000000,A=1.000000)" 5.0)
    (else
      (Variables|Default|SetObjectActivated true)
      (Rendering|Material|SetVectorParameterValue (Variables|Default|GetDMI) "color" (Variables|Default|GetActiveColor) :!class /Script/Engine.MaterialInstanceDynamic)
      (Default|CallActivate))))

(event EventBeginPlay
  (bind _interactable (Variables|Default|GetInteractable))
  ;[1 0.15 0 0.5] Object setup when game starts
  (Utilities|FlowControl|Sequence
    (:then_0
      ;;[1 0.15 0 0.5] Creates a material instance to change the color of the object
      (bind _returnvalue (Rendering|Material|CreateDynamicMaterialInstance _interactable 0 0 "DMI_Cube" :!class /Script/Engine.PrimitiveComponent))
      (bind _output_get (Variables|Default|SetDMI _returnvalue))
      (Rendering|Material|SetMaterial _interactable 0 _output_get))
    (:then_1
      ;;[1 0.15 0 0.5] Set state of object at start
      (Variables|Default|SetObjectActivated false)
      (Rendering|Material|SetVectorParameterValue (Variables|Default|GetDMI) "color" (Variables|Default|GetPL_InactiveColor) :!class /Script/Engine.MaterialInstanceDynamic))))

(fn ConstructionScript)

(fn IODeactivate)

(fn IsInteractable
  (return false))

(fn OnGrapple
  (params (InteractingPlayer :type Character%20Object%20Reference))
  (return "NewEnumerator3"))