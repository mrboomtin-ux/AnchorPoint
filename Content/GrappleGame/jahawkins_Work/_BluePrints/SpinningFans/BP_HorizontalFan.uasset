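; BP_HorizontalFan is a horizontal fan that spins continuously, alternating between its starting and slowed rotation speeds.
; BeginPlay runs an endless loop that switches CurrentRotSpeed on fixed three-second delays, calling ActivateFan to apply the slowed speed.
; Tick yaws the Pivot component by that speed scaled by delta time, so speed changes are instant rather than eased.
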(event Custom|ActivateFan
  (Variables|Default|SetCurrentRotSpeed (Variables|Default|GetSlowedRotSpeed)))

(event EventBeginPlay
  (Variables|Default|SetCurrentRotSpeed (Variables|Default|GetStartingRotSpeed) :!label _label)
  (Utilities|FlowControl|Delay 3.0)
  (CallFunction|ActivateFan)
  (Utilities|FlowControl|Delay 3.0)
  (goto _label))

(event EventTick
  (params (DeltaSeconds :type Float%20%28single-precision%29))
  (Transformation|AddLocalRotation (Variables|Default|GetPivot) (Math|Rotator|MakeRotator 0.0 0.0 (* DeltaSeconds (Variables|Default|GetCurrentRotSpeed))) false false))

(fn ConstructionScript
  (|CallParentFunction))