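; BP_VerticalFan is a spinning fan hazard that rotates around its pitch axis.
; BeginPlay sets the current rotation speed to the maximum and binds events to the InteractableObject's activate and deactivate hooks, though their handlers are not defined here.
; Tick applies a delta-time-scaled local pitch rotation to the Pivot at the current speed.
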(event EventBeginPlay
  (bind _interactableobject (Variables|Default|GetInteractableObject))
  (Utilities|FlowControl|Sequence
    (:then_0
      (Variables|Default|SetCurrentRotSpeed (Variables|Default|GetMaxRotSpeed)))
    (:then_1
      (EventDispatchers|BindEventtoActivate _interactableobject (EventDispatchers|CreateEvent :!event ReduceSpeed))
      (EventDispatchers|BindEventtoDeactivate _interactableobject (EventDispatchers|CreateEvent :!event BoostSpeed)))))

(event EventTick
  (params (DeltaSeconds :type Float%20%28single-precision%29))
  (Transformation|AddLocalRotation (Variables|Default|GetPivot) (Math|Rotator|MakeRotator 0.0 (* DeltaSeconds (Variables|Default|GetCurrentRotSpeed)) 0.0) false false))

(fn ConstructionScript
  (|CallParentFunction))