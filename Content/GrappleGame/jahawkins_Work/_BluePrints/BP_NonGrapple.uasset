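; BP_NonGrapple is a zone that blocks the player's grapple while they stand inside it and shows a NoGrappleZone widget.
; On begin and end overlap it checks the player's capsule and, while the zone is active, clears CanGrapple; leaving restores it and removes the widget.
; A linked Lever's activation fires DisableZone, switching the restriction off and restoring grappling.
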(event OnComponentBeginOverlap(Zone)
  (params (OverlappedComponent :type Primitive%20Component%20Object%20Reference) (OtherActor :type Actor%20Object%20Reference) (OtherComp :type Primitive%20Component%20Object%20Reference) (OtherBodyIndex :type Integer) (bFromSweep :type Boolean) (SweepResult :type Hit%20Result%20Structure%20%28by%20ref%29))
  (bind _player (Variables|Default|GetPlayer))
  ;[1 0.15 0 0.5] Search for player overlap
  (if (Class|PrimitiveComponent|IsOverlappingComponent (Variables|Default|GetZone) (Variables|/Script/Engine.Character|GetCapsuleComponent (Variables|Default|GetPlayer)))
    (if (Variables|Default|GetDisableGrapple)
      (Variables|/Game/GrappleGame/Progamers/_Blueprints/BP_GrappleCharacter.BP_GrappleCharacter_C|SetCanGrapple? _player false)
      ;[1 0.15 0 0.5] Handles UI for NoGrappleZone
      (UserInterface|Viewport|AddtoViewport (stale EventBeginPlay _returnvalue_2) 0))
    (else
      (Variables|/Game/GrappleGame/Progamers/_Blueprints/BP_GrappleCharacter.BP_GrappleCharacter_C|SetCanGrapple? _player true)
      (Widget|RemovefromParent (stale EventBeginPlay _returnvalue_2)))))

(event OnComponentEndOverlap(Zone)
  (params (OverlappedComponent :type Primitive%20Component%20Object%20Reference) (OtherActor :type Actor%20Object%20Reference) (OtherComp :type Primitive%20Component%20Object%20Reference) (OtherBodyIndex :type Integer))
  (bind _player (Variables|Default|GetPlayer))
  ;[1 0.15 0 0.5] Search for player overlap
  (if (Class|PrimitiveComponent|IsOverlappingComponent (Variables|Default|GetZone) (Variables|/Script/Engine.Character|GetCapsuleComponent (Variables|Default|GetPlayer)))
    (if (Variables|Default|GetDisableGrapple)
      (Variables|/Game/GrappleGame/Progamers/_Blueprints/BP_GrappleCharacter.BP_GrappleCharacter_C|SetCanGrapple? _player false)
      ;[1 0.15 0 0.5] Handles UI for NoGrappleZone
      (UserInterface|Viewport|AddtoViewport (stale EventBeginPlay _returnvalue_2) 0))
    (else
      (Variables|/Game/GrappleGame/Progamers/_Blueprints/BP_GrappleCharacter.BP_GrappleCharacter_C|SetCanGrapple? _player true)
      (Widget|RemovefromParent (stale EventBeginPlay _returnvalue_2)))))

(event Custom|DisableZone
  ;[1 0.15 0 0.5] Store reference to player and conencts lever to grapple zone
  (Variables|Default|SetDisableGrapple false)
  (Variables|/Game/GrappleGame/Progamers/_Blueprints/BP_GrappleCharacter.BP_GrappleCharacter_C|SetCanGrapple? (Variables|Default|GetPlayer) true))

(event EventBeginPlay
  ;[1 0.15 0 0.5] Store reference to player and conencts lever to grapple zone
  (bind _returnvalue (Actor|GetActorOfClass "/Game/GrappleGame/Progamers/_Blueprints/BP_GrappleCharacter.BP_GrappleCharacter_C"))
  (Variables|Default|SetPlayer _returnvalue)
  (EventDispatchers|BindEventtoActivate (Variables|Default|GetLever) (delegate Custom|DisableZone))
  ;[1 0.15 0 0.5] Create UI for NoGrappleZone
  (bind _returnvalue_2 (UserInterface|CreateWidget "/Game/GrappleGame/jahawkins_Work/_UI/WBP_NoGZone.WBP_NoGZone_C")))

(fn ConstructionScript)