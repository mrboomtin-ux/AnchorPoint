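; BP_Exit is a level exit trigger that loads the LevelComplete level when the player's grapple character enters it.
; BeginPlay caches the player character and a level manager reference, though the manager is not used further here.
; A box overlap opens the level only when the other component is that character's capsule.
; The construction script sizes the box from BoxShape, raises it by its Z value, and zeroes its relative rotation.
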(event OnComponentBeginOverlap(Box)
  (params (OverlappedComponent :type Primitive%20Component%20Object%20Reference) (OtherActor :type Actor%20Object%20Reference) (OtherComp :type Primitive%20Component%20Object%20Reference) (OtherBodyIndex :type Integer) (bFromSweep :type Boolean) (SweepResult :type Hit%20Result%20Structure%20%28by%20ref%29))
  (if (== OtherComp (Variables|/Script/Engine.Character|GetCapsuleComponent (Variables|Default|GetAs%20BP%20Grapple%20Character)))
    (Game|OpenLevel(byObjectReference) "/Game/GrappleGame/Progamers/_Blueprints/Levels/LevelComplete.LevelComplete")))

(event EventBeginPlay
  ;[0.15 0.15 0.15 0.5] Get reference to the Level Manager
  (bind _returnvalue (Actor|GetActorOfClass "/Game/GrappleGame/Progamers/_Blueprints/PuzzleMechanics/BP_LevelManager.BP_LevelManager_C"))
  (Variables|Default|SetLevelManagerRef _returnvalue)
  ;[0.15 0.15 0.15 0.5] player ref
  (bind _asbp_grapple_character (Utilities|Casting|CastToBP_GrappleCharacter (Game|GetPlayerCharacter 0)))
  (Variables|Default|SetAs%20BP%20Grapple%20Character _asbp_grapple_character))

(fn ConstructionScript
  (Transformation|AddLocalOffset (Variables|Default|GetBox) (Math|Vector|MakeVector 0.0 0.0 (.z (Variables|Default|GetBox%20Shape))) false false)
  (Components|Box|SetBoxExtent (Variables|Default|GetBox) (Variables|Default|GetBox%20Shape) true)
  (Transformation|SetRelativeRotation (Variables|Default|GetBox) "0, 0, 0" false false))